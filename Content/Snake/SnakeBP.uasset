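; Snake player Blueprint that moves steadily along world X and passes input state to its animation.
; On BeginPlay it caches the mesh's SnakeAnimBlueprint instance and sets it running, a step marked as temporary.
; Jump and MoveRight input only set jump and turn flags on that instance.
; Tick reads the running flag back from the anim instance to offset actor location by MovementSpeed scaled by delta time.
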(event `InputAction|Jump`
  (params (Key :type "Key Structure"))
  (bind _animationbp (`self.AnimationBP`))
  (:`Pressed`
    (set `/Game/Snake/SnakeAnimBlueprint.isJumping` true _animationbp))
  (:`Released`
    (set `/Game/Snake/SnakeAnimBlueprint.isJumping` false _animationbp)))

(event `InputAxis|MoveRight` :overrideparent false
  (params (AxisValue :type "Float (single-precision)"))
  (bind _animationbp (`self.AnimationBP`))
  (set `/Game/Snake/SnakeAnimBlueprint.isLeftTurning` (== AxisValue -1.0) _animationbp)
  (set `/Game/Snake/SnakeAnimBlueprint.isRightTurning` (== AxisValue 1.0) _animationbp))

(event `self.ReceiveBeginPlay`
  (bind _assnake_anim_blueprint (cast `/Game/Snake/SnakeAnimBlueprint` (`SkeletalMeshComponent.GetAnimInstance` (`self.Mesh`))))
  (set `self.AnimationBP` _assnake_anim_blueprint)
  ;[1 1 1] To be changed later
  (set `/Game/Snake/SnakeAnimBlueprint.isRunning` true (`self.AnimationBP`)))

(event `self.ReceiveTick`
  (params (DeltaSeconds :type "Float (single-precision)"))
  (bind (_returnvalue_x _returnvalue_y _returnvalue_z) (`KismetMathLibrary.BreakVector` (`self.K2_GetActorLocation`)))
  (if (`/Game/Snake/SnakeAnimBlueprint.isRunning` (`self.AnimationBP`))
    (`self.K2_SetActorLocation` (`KismetMathLibrary.MakeVector` (+ _returnvalue_x (* DeltaSeconds (`self.MovementSpeed`))) _returnvalue_y _returnvalue_z))))

(fn `UserConstructionScript`)