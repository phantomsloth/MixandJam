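; BP_ObstacleManager periodically spawns lane obstacles ahead of the player's snake.
; On BeginPlay it caches the SnakeBP player pawn and starts a looping timer whose 2–3 second interval is randomized once.
; Each tick of that timer randomly spawns a one-lane or two-lane obstacle actor at a fixed X offset from the snake mesh's current location.
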(event `self.ReceiveBeginPlay`
  (bind _assnake_bp (cast `/Game/Snake/SnakeBP` (`GameplayStatics.GetPlayerPawn` 0)))
  (set `self.SnakeReference` _assnake_bp)
  (`KismetSystemLibrary.K2_SetTimerDelegate` (delegate `CustomEvent_0`) (`KismetMathLibrary.RandomFloatInRange` 2.0 3.0) true))

(event `CustomEvent_0`
  (bind _y (.y (`SceneComponent.K2_GetComponentLocation` (`Character.Mesh` (`self.SnakeReference`)))))
  (bind _z (.z (`SceneComponent.K2_GetComponentLocation` (`Character.Mesh` (`self.SnakeReference`)))))
  (bind _returnvalue (+ (.x (`SceneComponent.K2_GetComponentLocation` (`Character.Mesh` (`self.SnakeReference`)))) 1500.0))
  (switch `int` (`KismetMathLibrary.RandomInteger` 2)
    (:`Default`
      (`|SpawnActorFromClass` "/Game/MixandJam/Core/Obstacles/BP_ObstaclesTwoLane.BP_ObstaclesTwoLane_C" (`KismetMathLibrary.MakeTransform` (`KismetMathLibrary.MakeVector` _returnvalue _y _z)) "Undefined" "OverrideRootScale" null null :!label _label))
    (:`0`
      (goto _label))
    (:`1`
      (`|SpawnActorFromClass` "/Game/MixandJam/Core/Obstacles/BP_ObstaclesOneLane.BP_ObstaclesOneLane_C" (`KismetMathLibrary.MakeTransform` (`KismetMathLibrary.MakeVector` _returnvalue _y _z)) "Undefined" "OverrideRootScale" null null))))

(fn `UserConstructionScript`)